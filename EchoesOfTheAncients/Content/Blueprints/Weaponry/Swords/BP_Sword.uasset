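; BP_Sword is a sword weapon Blueprint that can break and scatter Chaos destructible objects at a given location.
; Its CreateFields event applies two transient physics fields there: a radial falloff external cluster strain to fracture geometry, then a filtered radial vector linear force to push the pieces outward.
; Nothing in this graph calls the event, and the construction script only runs the parent's.
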(event `self.CreateFields`
  (params (FieldLocation :type "Vector Structure (by ref)"))
  (bind _fieldsystem (`self.FieldSystem`))
  (`FieldSystemComponent.ApplyPhysicsField` _fieldsystem true "Field_ExternalClusterStrain" null (`RadialFalloff.SetRadialFalloff` (`self.RadialFalloff`) 50000.0 0.8 1.0 0.0 50.0 FieldLocation "Field_FallOff_None"))
  (`FieldSystemComponent.ApplyPhysicsField` _fieldsystem true "Field_LinearForce" (`self.FieldSystemMetaDataFilter`) (`RadialVector.SetRadialVector` (`self.RadialVector`) 5000.0 FieldLocation)))

(fn `UserConstructionScript`
  (`parent.UserConstructionScript`))